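; Trigger box that sequences shockwave waves ("ondes de choc") and flags IsOverlapped when the first-person character enters.
; SequenceTest starts the SpawnerOndesDeChocs at the current Id, waits, counts the wave, then cycles Id through 0–3 and re-arms itself by timer using the wave's duration.
; A separate event spawns safe-zone pairs by Id.
; Nothing here starts the loop from the overlap, and older sequence logic sits disconnected.
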(event OnComponentBeginOverlap(CollisionComponent)
  (params (OverlappedComponent :type Primitive%20Component%20Object%20Reference) (OtherActor :type Actor%20Object%20Reference) (OtherComp :type Primitive%20Component%20Object%20Reference) (OtherBodyIndex :type Integer) (bFromSweep :type Boolean) (SweepResult :type Hit%20Result%20Structure%20%28by%20ref%29))
  (Utilities|Casting|CastToFirstPersonCharacter OtherActor)
  (Variables|Default|SetIsOverlapped true))

(event Custom|SequenceTest
  (bind _tempsentrespawn (Variables|Default|GetTempsEntreSpawn))
  (bind _outactors (Actor|GetAllActorsOfClass "/Game/Blueprints/SpawnerOndesDeChocs.SpawnerOndesDeChocs_C"))
  (Default|Commencement (Utilities|Array|Get(acopy) _outactors (Variables|Default|Getid)))
  (Utilities|FlowControl|Delay _tempsentrespawn)
  (Variables|Default|SetTemps (+ _tempsentrespawn (Variables|/Game/Blueprints/SpawnerOndesDeChocs.SpawnerOndesDeChocs_C|GetDurée%20Onde (Utilities|Array|Get(acopy) _outactors (Variables|Default|Getid)))))
  (Variables|Default|SetVagues (+ (Variables|Default|GetVagues) 1.0))
  (CallFunction|AjoutId))

(event Custom|AjoutId
  (if (< (Variables|Default|Getid) 3)
    (Variables|Default|Setid (+ (Variables|Default|Getid) 1))
    (else
      (Variables|Default|Setid (- (Variables|Default|Getid) (Variables|Default|Getid)))))
  (CallFunction|Essai))

(event Custom|Essai
  (Utilities|Time|SetTimerbyEvent (delegate Custom|SequenceTest) (Variables|Default|GetTemps) (>= (Variables|Default|GetVagues) (Variables|Default|GetVaguesMax))))

(event Custom|ZonesSafesSeq01
  (if (== (Variables|Default|Getid) 0)
    (bind _outactors (Actor|GetAllActorsOfClass "/Game/Blueprints/SpawnZonesSafes.SpawnZonesSafes_C"))
    (Default|Spawner (Utilities|Array|Get(acopy) _outactors))
    (elif (== (Variables|Default|Getid) 1)
      (bind _outactors_2 (Actor|GetAllActorsOfClass "/Game/Blueprints/SpawnZonesSafes.SpawnZonesSafes_C"))
      (Default|Spawner (Utilities|Array|Get(acopy) _outactors_2 2)))))

(fn ConstructionScript)

(fn Sequence)