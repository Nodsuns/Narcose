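; OndesDeChocs is a shockwave actor that travels in a straight line and destroys itself after a set duration.
; Duree stores the lifetime and calls Spawn, which waits that delay, sets DelayComplet and destroys the actor.
; Each Tick records the Box's world scale and moves the actor along the Box's up vector by Vitesse, set through VitesseOnde, without sweep or delta-time scaling.
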(event Custom|Spawn
  ;[1 1 1] Durée d'une Onde
  (Utilities|FlowControl|Delay (Variables|Default|GetDelay))
  (Variables|Default|SetDelayComplet true)
  (Actor|DestroyActor))

(event EventTick
  (params (DeltaSeconds :type Float%20%28single-precision%29))
  ;[1 1 1] Avancement Onde
  (Variables|Default|SetScale (Transformation|GetWorldScale (Variables|Default|GetBox)))
  (Transformation|SetActorLocation (+ (Transformation|GetActorLocation) (* (Math|Vector|GetUpVector (Transformation|GetWorldRotation (Variables|Default|GetBox))) (Variables|Default|GetVitesse))) false false))

(fn ConstructionScript)

(fn Duree
  (params (delay :type Float%20%28single-precision%29))
  (Variables|Default|SetDelay delay)
  (CallFunction|Spawn))

(fn VitesseOnde
  (params (Vitesse :type Integer))
  (Variables|Default|SetVitesse Vitesse))