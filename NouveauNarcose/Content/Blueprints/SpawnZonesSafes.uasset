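; SpawnZonesSafes is a spawner actor that creates safe zones (ZonesSafes) in the level.
; Its Spawner event spawns one at the Box component's world transform, then passes the Désactiver flag to Activer and copies it into ZoneSafesActives.
; Désactivation sets that flag false and Réactivation sets it true, so despite its name, true corresponds to reactivation.
; Neither toggle event updates zones already spawned.
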(event Custom|Spawner
  (bind _désactiver (Variables|Default|GetDésactiver))
  (bind _returnvalue (Game|SpawnActorfromClass "/Game/Blueprints/ZonesSafes.ZonesSafes_C" (Math|Transform|MakeTransform (Transformation|GetWorldLocation (Variables|Default|GetBox)) (Transformation|GetWorldRotation (Variables|Default|GetBox)) (Transformation|GetWorldScale (Variables|Default|GetBox))) "Undefined" 0 0))
  (Default|Activer _returnvalue _désactiver)
  (Variables|/Game/Blueprints/ZonesSafes.ZonesSafes_C|SetZoneSafesActives _returnvalue _désactiver))

(event Custom|Désactivation
  (Variables|Default|SetDésactiver false))

(event Custom|Réactivation
  (Variables|Default|SetDésactiver true))

(fn ConstructionScript)