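; Mine is a proximity trap actor that kills the player when they enter its detection zone.
; An overlap by FirstPersonCharacter waits half a second, then spawns an explosion emitter at the mine and plays a 2D sound.
; It then disables the actor's input for player 0, shows the mouse cursor, displays the Mort death widget and destroys itself.
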(event OnComponentBeginOverlap(DetectionZone)
  (params (OverlappedComponent :type Primitive%20Component%20Object%20Reference) (OtherActor :type Actor%20Object%20Reference) (OtherComp :type Primitive%20Component%20Object%20Reference) (OtherBodyIndex :type Integer) (bFromSweep :type Boolean) (SweepResult :type Hit%20Result%20Structure%20%28by%20ref%29))
  (bind _returnvalue (Game|GetPlayerController 0))
  (Utilities|Casting|CastToFirstPersonCharacter OtherActor)
  (Utilities|FlowControl|Delay 0.5)
  (Effects|SpawnEmitteratLocation 0 (Transformation|GetActorLocation))
  (Audio|PlaySound2D 0 1.0 1.0 0.0 0 0)
  (Input|DisableInput _returnvalue)
  (Variables|/Script/Engine.PlayerController|SetbShowMouseCursor _returnvalue true)
  (bind _returnvalue_2 (UserInterface|CreateWidget "/Game/Interface/Mort.Mort_C"))
  (UserInterface|Viewport|AddtoViewport _returnvalue_2 0)
  (Actor|DestroyActor))

(fn ConstructionScript)