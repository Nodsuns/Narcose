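; Spawner actor that unleashes a shockwave (OndesDeChocs) announced by a monster scream.
; Commencement plays the scream and shakes the camera at the player's position, then waits briefly and arms a one-shot timer.
; The timer's Spawner event spawns the wave at the root's transform with the chosen scale, then passes it duration and speed.
; invalidationTimer cancels a pending spawn.
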(event Custom|Spawner
  (bind _durée_onde (Variables|Default|GetDurée%20Onde))
  (bind _vitesse (Variables|Default|Getvitesse))
  (bind _output_get (Variables|Default|SetScaleOnde (Variables|Default|GetScaleChoisie)))
  (bind _returnvalue (Game|SpawnActorfromClass "/Game/Blueprints/OndesDeChocs.OndesDeChocs_C" (Math|Transform|MakeTransform (Transformation|GetWorldLocation (Variables|Default|GetDefaultSceneRoot)) (Transformation|GetWorldRotation (Variables|Default|GetDefaultSceneRoot)) _output_get) "Undefined" 0 0))
  (Default|Duree _returnvalue _durée_onde)
  (Variables|/Game/Blueprints/OndesDeChocs.OndesDeChocs_C|SetDelay _returnvalue _durée_onde)
  (Default|VitesseOnde _returnvalue _vitesse)
  (Variables|/Game/Blueprints/OndesDeChocs.OndesDeChocs_C|SetVitesse _returnvalue _vitesse))

(event Custom|Commencement
  (Audio|PlaySoundatLocation "/Game/Sound/Créature/HurlementMonstre.HurlementMonstre" (Transformation|GetWorldLocation (Variables|Default|GetDefaultSceneRoot)) "0, 0, 0" 1.0 1.0 0.0 0 0 0)
  (bind _asfirst_person_character (Utilities|Casting|CastToFirstPersonCharacter (Game|GetPlayerCharacter 0)))
  (Camera|PlayWorldCameraShake "/Game/Camera/ShakeCamera.ShakeCamera_C" (Transformation|GetActorLocation _asfirst_person_character) 0.0 5e+02 1.0 true)
  (Utilities|FlowControl|Delay 1.0)
  (bind _returnvalue (Utilities|Time|SetTimerbyEvent (delegate Custom|Spawner) (Variables|Default|GetVitesseDeSpawn))))

(event Custom|invalidationTimer
  (Utilities|Time|ClearandInvalidateTimerbyHandle (stale Custom|Commencement _returnvalue)))

(fn ConstructionScript
  (Variables|Default|SetScaleChoisie (Variables|Default|GetScaleChoisie)))