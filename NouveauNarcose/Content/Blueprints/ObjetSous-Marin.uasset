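; Submarine object that starts a blinking beacon with a beep once the OndePerso character enters its trigger box.
; The box overlap starts a looping one-second timer that calls Bip.
; Bip toggles the point light's visibility and plays the beep sound at the light's location each time it turns on.
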(event OnComponentBeginOverlap(Box)
  (params (OverlappedComponent :type Primitive%20Component%20Object%20Reference) (OtherActor :type Actor%20Object%20Reference) (OtherComp :type Primitive%20Component%20Object%20Reference) (OtherBodyIndex :type Integer) (bFromSweep :type Boolean) (SweepResult :type Hit%20Result%20Structure%20%28by%20ref%29))
  (Utilities|Casting|CastToOndePerso OtherActor)
  (Utilities|Time|SetTimerbyEvent (delegate Custom|Bip) 1.0 true))

(event Custom|Bip
  (bind _pointlight (Variables|Default|GetPointLight))
  (if (Variables|Default|GetVisibilityLight)
    (bind _output_get (Variables|Default|SetVisibilityLight false))
    (Rendering|SetVisibility (Variables|Default|GetPointLight) _output_get false)
    (else
      (bind _output_get_2 (Variables|Default|SetVisibilityLight true))
      (Rendering|SetVisibility _pointlight _output_get_2 false)
      (Audio|PlaySoundatLocation "/Game/Sound/BipObjetSous-Marin.BipObjetSous-Marin" (Transformation|GetWorldLocation _pointlight) "0, 0, 0" 1.0 1.0 0.0 0 0 0))))

(fn ConstructionScript)