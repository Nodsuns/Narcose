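; Checkpoint actor that saves the game when the FirstPersonCharacter overlaps its CheckPoint component.
; It loads the existing CheckpointSaveGame from its slot, or creates one if none exists.
; It stores a transform 200 units above the actor, with zero rotation and unit scale, then writes the slot and prints the saved transform.
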(event OnComponentBeginOverlap(CheckPoint)
  (params (OverlappedComponent :type Primitive%20Component%20Object%20Reference) (OtherActor :type Actor%20Object%20Reference) (OtherComp :type Primitive%20Component%20Object%20Reference) (OtherBodyIndex :type Integer) (bFromSweep :type Boolean) (SweepResult :type Hit%20Result%20Structure%20%28by%20ref%29))
  (bind _checkpointsavename (Variables|Default|GetCheckpointSaveName))
  ;[1 1 1] Sauvegarde Checkpoint
  (Utilities|Casting|CastToFirstPersonCharacter OtherActor)
  (bind _returnvalue (SaveGame|DoesSaveGameExist _checkpointsavename))
  (if _returnvalue
    (bind _returnvalue_2 (SaveGame|LoadGamefromSlot _checkpointsavename))
    (bind _ascheckpoint_save_game (Utilities|Casting|CastToCheckpointSaveGame _returnvalue_2))
    (Variables|Default|SetSaveGameReference _ascheckpoint_save_game)
    (else
      (bind _returnvalue_3 (SaveGame|CreateSaveGameObject "/Game/Blueprints/Checkpoint/CheckpointSaveGame.CheckpointSaveGame_C"))
      (Variables|Default|SetSaveGameReference _returnvalue_3)))
  (bind _output_get (Variables|/Game/Blueprints/Checkpoint/CheckpointSaveGame.CheckpointSaveGame_C|SetCheckpoint (Variables|Default|GetSaveGameReference) (Math|Transform|MakeTransform (+ (.location (Transformation|GetActorTransform)) "0, 0,200.000000"))))
  (SaveGame|SaveGametoSlot (Variables|Default|GetSaveGameReference) (Variables|Default|GetCheckpointSaveName))
  (Development|PrintString (Utilities|String|Append "Saved game." "Transform : " (Utilities|String|ToString(Transform) _output_get))))

(fn ConstructionScript)