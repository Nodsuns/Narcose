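; Oxygen bottle actor that gradually refills the first-person character's oxygen while its interaction box overlaps the bottle.
; A quarter-second timer transfers oxygen, drains the bottle, then re-runs the checks for an empty bottle, transfer cap or full player, re-setting itself.
; Ending the overlap or reaching the player's maximum clears the timer.
; Tick updates a widget progress bar with the remaining oxygen.
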(event OnComponentEndOverlap(Bouteille)
  (params (OverlappedComponent :type Primitive%20Component%20Object%20Reference) (OtherActor :type Actor%20Object%20Reference) (OtherComp :type Primitive%20Component%20Object%20Reference) (OtherBodyIndex :type Integer))
  ;[1 1 1] Déclic
  (Utilities|Casting|CastToBoxInteractionPerso OtherActor)
  ;[0 1 0.4984] Ajout Oxygene
  (Utilities|Time|ClearandInvalidateTimerbyHandle (stale Custom|PrendreDeLOxygene _returnvalue)))

(event Custom|PrendreDeLOxygene
  (bind _ajoutdoxygene (Variables|Default|GetAjoutDOxygene))
  ;[0 1 0.4984] Ajout Oxygene
  (Variables|/Game/FirstPersonBP/Blueprints/FirstPersonCharacter.FirstPersonCharacter_C|SetOxygene (stale _asfirst_person_character) (+ (Variables|/Game/FirstPersonBP/Blueprints/FirstPersonCharacter.FirstPersonCharacter_C|GetOxygene (stale _asfirst_person_character)) _ajoutdoxygene))
  (Variables|Default|SetOxygeneAjoute (+ (Variables|Default|GetOxygeneAjoute) _ajoutdoxygene))
  (Variables|Default|SetOxygeneDansBouteille (- (Variables|Default|GetOxygeneDansBouteille) 1.66))
  (if (<= (Variables|Default|GetOxygeneDansBouteille) 0.0)
    (Development|PrintString "Vide" :!label _label)
    (elif (>= (Variables|Default|GetOxygeneAjoute) 3e+02)
      (goto _label)
      (else
        (bind _asfirst_person_character (Utilities|Casting|CastToFirstPersonCharacter (Game|GetPlayerCharacter 0)))
        (if (< (Variables|/Game/FirstPersonBP/Blueprints/FirstPersonCharacter.FirstPersonCharacter_C|GetOxygene _asfirst_person_character) 5e+02)
          (bind _returnvalue (Utilities|Time|SetTimerbyEvent (delegate Custom|PrendreDeLOxygene) 0.25 (< (Variables|Default|GetOxygeneAjoute) 3e+02)))
          (else
            (Development|PrintString "Oxygene au max")
            (Utilities|Time|ClearandInvalidateTimerbyHandle _returnvalue)))))))

(event EventTick
  (params (DeltaSeconds :type Float%20%28single-precision%29))
  ;[1 1 1] Barre d'oxygène
  (bind _asbouteille_vie (Utilities|Casting|CastToBouteilleVie (UserInterface|GetUserWidgetObject (Variables|Default|GetBouteilleVieW))))
  (Progress|SetPercent (Variables|/Game/Interfaces/BouteilleVie.BouteilleVie_C|GetVieBouteille _asbouteille_vie) (/ (Variables|Default|GetOxygeneDansBouteille) (Variables|Default|GetMaxOxygene))))

(event Collision|EventActorBeginOverlap
  (params (OtherActor :type Actor%20Object%20Reference))
  ;[0 1 0.4984] Ajout Oxygene
  (Utilities|Casting|CastToBoxInteractionPerso OtherActor)
  (if (<= (Variables|Default|GetOxygeneDansBouteille) 0.0)
    (Development|PrintString "Vide" :!label _label)
    (elif (>= (Variables|Default|GetOxygeneAjoute) 3e+02)
      (goto _label)
      (else
        (bind _asfirst_person_character (Utilities|Casting|CastToFirstPersonCharacter (Game|GetPlayerCharacter 0)))
        (if (< (Variables|/Game/FirstPersonBP/Blueprints/FirstPersonCharacter.FirstPersonCharacter_C|GetOxygene _asfirst_person_character) 5e+02)
          (bind _returnvalue (Utilities|Time|SetTimerbyEvent (delegate Custom|PrendreDeLOxygene) 0.25 (< (Variables|Default|GetOxygeneAjoute) 3e+02)))
          (else
            (Development|PrintString "Oxygene au max")
            (Utilities|Time|ClearandInvalidateTimerbyHandle _returnvalue)))))))

(fn ConstructionScript)