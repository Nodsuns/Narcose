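; Energy cell pickup that fully restores the first-person player's energy.
; A looping timer toggles the Lumieree component's visibility every half second to make it blink.
; When a BoxInteractionPerso actor overlaps the Ener component, it casts player character 0 to FirstPersonCharacter, raises Energie to EnergieMax, then destroys itself.
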(event OnComponentBeginOverlap(Ener)
  (params (OverlappedComponent :type Primitive%20Component%20Object%20Reference) (OtherActor :type Actor%20Object%20Reference) (OtherComp :type Primitive%20Component%20Object%20Reference) (OtherBodyIndex :type Integer) (bFromSweep :type Boolean) (SweepResult :type Hit%20Result%20Structure%20%28by%20ref%29))
  (Utilities|Casting|CastToBoxInteractionPerso OtherActor)
  (bind _asfirst_person_character (Utilities|Casting|CastToFirstPersonCharacter (Game|GetPlayerCharacter 0)))
  (Variables|/Game/FirstPersonBP/Blueprints/FirstPersonCharacter.FirstPersonCharacter_C|SetEnergie _asfirst_person_character (+ (Variables|/Game/FirstPersonBP/Blueprints/FirstPersonCharacter.FirstPersonCharacter_C|GetEnergie _asfirst_person_character) (- (Variables|/Game/FirstPersonBP/Blueprints/FirstPersonCharacter.FirstPersonCharacter_C|GetEnergieMax _asfirst_person_character) (Variables|/Game/FirstPersonBP/Blueprints/FirstPersonCharacter.FirstPersonCharacter_C|GetEnergie _asfirst_person_character))))
  (Actor|DestroyActor))

(event Custom|Clignotement
  (Rendering|ToggleVisibility (Variables|Default|GetLumieree) false))

(event EventBeginPlay
  (Utilities|Time|SetTimerbyEvent (delegate Custom|Clignotement) 0.5 true))

(fn ConstructionScript)