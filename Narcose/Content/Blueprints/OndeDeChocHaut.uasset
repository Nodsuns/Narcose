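; OndeDeChocHaut is a shockwave actor that travels along the up vector of its Onde component and removes itself after a short lifetime.
; Tick offsets the actor by Vitesse each frame without sweep or delta-time scaling, so its speed depends on frame rate.
; BeginPlay starts a one-shot timer on the Choc event, which is empty, then destroys the actor after a delay.
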(event Custom|Choc
  ;[1 1 1] Durée d'une Onde
)

(event EventTick
  (params (DeltaSeconds :type Float%20%28single-precision%29))
  ;[1 1 1] Avancement Onde
  (Transformation|SetActorLocation (+ (Transformation|GetActorLocation) (* (Math|Vector|GetUpVector (Transformation|GetWorldRotation (Variables|Default|GetOnde))) (Variables|Default|GetVitesse))) false false))

(event EventBeginPlay
  ;[1 1 1] Durée d'une Onde
  (Utilities|Time|SetTimerbyEvent (delegate Custom|Choc) 0.3)
  (Utilities|FlowControl|Delay 2.0)
  (Actor|DestroyActor (Components|GetOwner (Variables|Default|GetOnde))))

(fn ConstructionScript)