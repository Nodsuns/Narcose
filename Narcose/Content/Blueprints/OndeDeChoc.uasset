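; Shockwave actor ("onde de choc") that advances along an offset and destroys itself after a two-second delay.
; BeginPlay sets a short timer for Choc, which stores the actor's location and plays a timeline.
; The timeline lerps the Onde component's world location from that start by EndPoint, without sweep.
; Each timeline update feeds back into the timer and destroy-delay chain, re-arming the Choc timer.
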(event Custom|Choc
  ;[1 1 1] Avancement Onde
  (Variables|Default|SetStartPoint (Transformation|GetActorLocation))
  (bind _newtrack_0 (Timeline|Timeline_0 Play)
    (:Update
      (Transformation|SetWorldLocation (Variables|Default|GetOnde) (Math|Vector|Lerp(Vector) (Variables|Default|GetStartPoint) (+ (Variables|Default|GetStartPoint) (Variables|Default|GetEndPoint)) _newtrack_0) false false)
      ;[1 1 1] Durée d'une Onde
      (Utilities|Time|SetTimerbyEvent (delegate Custom|Choc) 0.3)
      (Utilities|FlowControl|Delay 2.0)
      (Actor|DestroyActor (Components|GetOwner (Variables|Default|GetOnde))))))

(event EventBeginPlay
  ;[1 1 1] Durée d'une Onde
  (Utilities|Time|SetTimerbyEvent (delegate Custom|Choc) 0.3)
  (Utilities|FlowControl|Delay 2.0)
  (Actor|DestroyActor (Components|GetOwner (Variables|Default|GetOnde))))

(fn ConstructionScript)